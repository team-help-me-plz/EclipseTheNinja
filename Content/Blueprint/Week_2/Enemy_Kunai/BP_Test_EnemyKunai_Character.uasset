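; Test enemy kunai character Blueprint built on side-scrolling character controls.
; Touch events forward interact, thumbstick movement and jump to the character's Do functions, with jump start also triggering a drop when the thumbstick's X axis points far enough negative.
; The attack input event is empty, and the GAS call that activates the GA_ThrowKunai ability is disconnected, so it never runs.
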(event Input|EnhancedActionEvents|EnhancedInputActionIA_Attack
  (params (ActionValue :type Boolean) (ElapsedSeconds :type Float%20%28double-precision%29) (TriggeredSeconds :type Float%20%28double-precision%29) (InputAction :type Input%20Action%20Object%20Reference :default "/Game/Input/IA_Attack.IA_Attack")))

(event EventPrimaryThumbstick
  (params (Axis :type Vector%202D%20Structure))
  ;[1 1 1] Touch controls for Third Person SideScrolling Character
  (Class|PlayerCharacter|DoMove (.y Axis)))

(event EventTouchJumpStart
  ;[1 1 1] Touch controls for Third Person SideScrolling Character
  (if (< (.x (stale EventPrimaryThumbstick Axis)) -0.5)
    (Class|PlayerCharacter|DoDrop (* (.x (stale EventPrimaryThumbstick Axis)) -1.0)))
  (Class|PlayerCharacter|DoJumpStart))

(event EventTouchJumpEnd
  ;[1 1 1] Touch controls for Third Person SideScrolling Character
  (Class|PlayerCharacter|DoJumpEnd))

(event EventTouchInteractStart
  ;[1 1 1] Touch controls for Third Person SideScrolling Character
  (Class|PlayerCharacter|DoInteract))

(fn ConstructionScript)