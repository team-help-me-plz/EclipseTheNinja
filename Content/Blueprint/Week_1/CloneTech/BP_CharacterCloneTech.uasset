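; Side-scrolling character Blueprint that maps touch controls to character actions.
; Touch and thumbstick events forward to interact, move and jump functions that are defined outside this graph, with movement driven by the thumbstick's Y axis.
; On jump press, a thumbstick X below a negative threshold also calls a drop with the negated value before starting the jump.
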(event EventPrimaryThumbstick
  (params (Axis :type Vector%202D%20Structure))
  ;[1 1 1] Touch controls for Third Person SideScrolling Character
  (Class|SideScrollingCharacter|DoMove (.y Axis)))

(event EventTouchJumpStart
  ;[1 1 1] Touch controls for Third Person SideScrolling Character
  (if (< (.x (stale EventPrimaryThumbstick Axis)) -0.5)
    (Class|SideScrollingCharacter|DoDrop (* (.x (stale EventPrimaryThumbstick Axis)) -1.0)))
  (Class|SideScrollingCharacter|DoJumpStart))

(event EventTouchJumpEnd
  ;[1 1 1] Touch controls for Third Person SideScrolling Character
  (Class|SideScrollingCharacter|DoJumpEnd))

(event EventTouchInteractStart
  ;[1 1 1] Touch controls for Third Person SideScrolling Character
  (Class|SideScrollingCharacter|DoInteract))

(fn ConstructionScript)