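; BP_SwitchDoor is a puzzle map door that slides between closed and open positions based on its Open flag.
; BeginPlay records the starting location as the closed position.
; Each Tick eases OpenAlpha toward open or closed with FInterpTo at OpenSpeed, then lerps the actor between that start and the start plus OpenOffset, without sweep.
; The file itself contains no logic that changes Open.
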(event EventBeginPlay
  (Variables|MapGameplay|SetStartLocation (Transformation|GetActorLocation)))

(event EventTick
  (params (DeltaSeconds :type Float%20%28single-precision%29))
  (bind _startlocation (Variables|MapGameplay|GetStartLocation))
  (Variables|MapGameplay|SetOpenAlpha (Math|Interpolation|FInterpTo (Variables|MapGameplay|GetOpenAlpha) (Math|Float|SelectFloat 1.0 0.0 (Variables|MapGameplay|GetbOpen)) DeltaSeconds (Variables|MapGameplay|GetOpenSpeed)))
  (Transformation|SetActorLocation (Math|Vector|Lerp(Vector) _startlocation (+ _startlocation (Variables|MapGameplay|GetOpenOffset)) (Variables|MapGameplay|GetOpenAlpha)) false false))

(fn ConstructionScript)