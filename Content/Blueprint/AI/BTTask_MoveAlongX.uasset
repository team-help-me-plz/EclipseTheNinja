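; Behavior tree task that walks an Enemy pawn along the X axis to the X of a blackboard vector key.
; Each tick it calls the enemy's MoveAlongX at a set speed, pausing during hit reactions and waiting until the enemy is ready for AI.
; It succeeds within a small X tolerance, fails on a dead or invalid enemy, and stops horizontal movement on arrival or abort.
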(event EventReceiveExecuteAI
  (params (OwnerController :type AI%20Controller%20Object%20Reference) (ControlledPawn :type Pawn%20Object%20Reference))
  ;[0.15 0.15 0.15 0.5] ReceiveExecuteAI
  (bind _asenemy (Utilities|Casting|CastToEnemy ControlledPawn)
    (:then
      (Variables|Default|SetEnemyRef _asenemy))
    (:CastFailed
      (AI|BehaviorTree|FinishExecute false))))

(event EventReceiveTickAI
  (params (OwnerController :type AI%20Controller%20Object%20Reference) (ControlledPawn :type Pawn%20Object%20Reference) (DeltaSeconds :type Float%20%28single-precision%29))
  (bind _keyselector (Variables|Default|GetKeySelector))
  (bind _returnvalue (Class|BTFunctionLibrary|GetBlackboardValueasVector _keyselector))
  (bind _x (Math|Vector|BreakVector _returnvalue))
  ;[0.15 0.15 0.15 0.5] ReceiveTickAI
  (if (Utilities|IsValid (Variables|Default|GetEnemyRef))
    (if (Class|Enemy|IsDead (Variables|Default|GetEnemyRef))
      (AI|BehaviorTree|FinishExecute false)
      (elif (Class|Enemy|IsReadyforAI (Variables|Default|GetEnemyRef))
        (if (Class|Enemy|IsPlayingHitReaction (Variables|Default|GetEnemyRef))
          (Class|Enemy|StopHorizontalMovement (Variables|Default|GetEnemyRef))
          (elif (<= (Math|Float|Absolute(Float) (- _x (.X (Math|Vector|BreakVector (Transformation|GetActorLocation (Variables|Default|GetEnemyRef)))))) 5.0)
            (Class|Enemy|StopHorizontalMovement (Variables|Default|GetEnemyRef))
            (AI|BehaviorTree|FinishExecute true)
            (else
              (Class|Enemy|MoveAlongX (Variables|Default|GetEnemyRef) _x (Variables|Default|GetMoveSpeed) DeltaSeconds))))))
    (else
      (AI|BehaviorTree|FinishExecute false))))

(event EventReceiveAbortAI
  (params (OwnerController :type AI%20Controller%20Object%20Reference) (ControlledPawn :type Pawn%20Object%20Reference))
  ;[0.15 0.15 0.15 0.5] ReceiveAbortAI
  (if (Utilities|IsValid (Variables|Default|GetEnemyRef))
    (Class|Enemy|StopHorizontalMovement (Variables|Default|GetEnemyRef))
    (Class|BTTaskBlueprintBase|FinishAbort)
    (else
      (Class|BTTaskBlueprintBase|FinishAbort))))